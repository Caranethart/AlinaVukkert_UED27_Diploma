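; Base enemy pawn that spots and chases the player, takes damage and attacks through health and attack action components.
; PawnSensing sightings start AIMoveTo and one-shot chase audio, with a retriggerable delay clearing sight and Tick fading the audio out.
; Damage lowers health, then alerts the AI controller or runs StartDeath, which triggers the attack action component.
; A target-death check clears the blackboard sight flag, and Tick draws patrol state as debug text.
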(event OnSeePawn(PawnSensing)
  (params (Pawn :type Pawn%20Object%20Reference))
  (bind _asbp_third_person_character (Utilities|Casting|CastToBP_ThirdPersonCharacter Pawn))
  (Utilities|FlowControl|Sequence
    (:then_0
      (Variables|Default|SetCanSeePlayer true)
      (AI|AIMoveTo self "0, 0, 0" _asbp_third_person_character 5.0 false
        (:then
          (Utilities|FlowControl|DoOnce false
            (:Completed
              (Audio|Components|Audio|Play (Variables|Default|GetAudio) 0.0))))))
    (:then_1
      (Utilities|FlowControl|RetriggerableDelay 0.6)
      (Variables|Default|SetCanSeePlayer false))))

(event EventBeginPlay
  (Utilities|FlowControl|Sequence
    (:then_0
      (bind _returnvalue (AddComponent|AddAudioComponent false))
      (Audio|Components|Audio|Stop _returnvalue)
      (Variables|Default|SetAudio _returnvalue))
    (:then_1
      (EventDispatchers|BindEventtoOnTakeAnyDamage (EventDispatchers|CreateEvent :!event ApplyDamage)))))

(event EventTick
  (params (DeltaSeconds :type Float%20%28single-precision%29))
  (if (Variables|Default|GetCanSeePlayer)
    (Rendering|Debug|DrawDebugString (+ (Transformation|GetWorldLocation (Variables|Collision|GetCapsuleComponent)) "0.000000,0.000000,20.000000") (Utilities|String|ToString(Text) (Utilities|Text|FormatText "{CurrentPatrolState} " (Utilities|String|EnumtoString (Variables|/Game/Components/BPAC_AIPatrollingManager.BPAC_AIPatrollingManager_C|GetPatrolState (Variables|Default|GetBPAC_AIPatrooling))))) 0 "(R=0.000000,G=0.149960,B=0.122139,A=1.000000)")
    (else
      (Utilities|FlowControl|Delay 0.4)
      (if (not (Variables|Default|GetCanSeePlayer))
        (Audio|Components|Audio|FadeOut (Variables|Default|GetAudio) 5.0 0.0 "Linear" :!class /Script/Engine.AudioComponent)
        (Utilities|FlowControl|DoOnce false) ; enters at Reset
      ))))

(fn ConstructionScript)

(fn ApplyDamage
  (params (DamagedActor :type Actor%20Object%20Reference) (Damage :type Float%20%28single-precision%29) (DamageType :type Damage%20Type%20Object%20Reference) (InstigatedBy :type Controller%20Object%20Reference) (DamageCauser :type Actor%20Object%20Reference))
  (Default|DecreaseValue (Variables|Default|GetBPAC_Health) (Math|Float|Truncate Damage))
  (if (> (Default|GetCurrentValue (Variables|Default|GetBPAC_Health)) 0)
    (bind _asbp_enemy_aicontroller (Utilities|Casting|CastToBP_EnemyAIController (AI|GetAIController self)))
    (Default|AttackedbyPlayer _asbp_enemy_aicontroller)
    (else
      (CallFunction|StartDeath))))

(fn StartDeath
  (if (not (Variables|Default|GetIsDead))
    (Default|StartAction (Variables|Default|GetBPAC_AttackAction))
    (Variables|Default|SetIsDead true)))

(fn AttackPlayer
  (params (AttackingActor :type Actor%20Object%20Reference))
  (Default|StartAction (Variables|Default|GetBPAC_AttackAction) AttackingActor))

(fn CheckIsTargetDead
  (if (<= (Default|GetCurrentValue (Actor|GetComponentbyClass (Game|GetPlayerCharacter 0) "/Game/Components/BPAC_Health.BPAC_Health_C")) 0)
    (AI|Components|Blackboard|SetValueasBool (AI|GetBlackboard 0) (Utilities|Name|MakeLiteralName "CanSeePlayer") false)
    (Variables|Default|SetIsAttacking false)
    (return true)
    (else
      (return false))))