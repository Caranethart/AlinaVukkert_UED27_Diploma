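; BP_DoorAuto is a door that opens automatically when an actor enters its collision box and closes after a delay.
; On overlap it branches on door state: Closed opens directly, while Locked first attempts an unlock with the overlapping actor and opens only on success.
; Leaving the box while Opened starts a one-shot close timer, cleared when the door opens again; TryClose wraps the Close call.
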(event OnComponentBeginOverlap(BoxCollision)
  (params (OverlappedComponent :type Primitive%20Component%20Object%20Reference) (OtherActor :type Actor%20Object%20Reference) (OtherComp :type Primitive%20Component%20Object%20Reference) (OtherBodyIndex :type Integer) (bFromSweep :type Boolean) (SweepResult :type Hit%20Result%20Structure%20%28by%20ref%29))
  (Utilities|SwitchCurrentState
    (:Closed
      (bind _success (CallFunction|Open :!label _label))
      (Utilities|Time|ClearandInvalidateTimerbyHandle (Variables|Default|GetDelayTimer)))
    (:Locked
      (bind _success_2 (CallFunction|SetIsLocked OtherActor false))
      (if _success_2
        (goto _label)))))

(event OnComponentEndOverlap(BoxCollision)
  (params (OverlappedComponent :type Primitive%20Component%20Object%20Reference) (OtherActor :type Actor%20Object%20Reference) (OtherComp :type Primitive%20Component%20Object%20Reference) (OtherBodyIndex :type Integer))
  (Utilities|SwitchCurrentState
    (:Opened
      (bind _returnvalue (Utilities|Time|SetTimerbyEvent (EventDispatchers|CreateEvent :!event TryClose) (Variables|Default|GetCloseDelayDuration)))
      (Variables|Default|SetDelayTimer _returnvalue))))

(fn ConstructionScript
  (|CallParentFunction))

(fn TryClose
  (CallFunction|Close))