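; Base door Blueprint that swings open and closed and can be locked, with a stub Interact that returns false.
; An Opened, Closed, Locked or Transition state gates Open and Close, which can reverse a swing midway.
; A duration-scaled timeline drives Animate to yaw DoorRotator, which the construction script also uses to pose the initial state.
; SetIsLocked switches between Closed and Locked only when the BPACLock component accepts the actor's request.
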(event EventBeginPlay
  (Components|Timeline|SetPlayRate (Variables|Default|GetDoorTimeline) (Math|Float|SafeDivide (Components|Timeline|GetTimelineLength (Variables|Default|GetDoorTimeline)) (Variables|Default|GetAnimationDuration))))

(fn ConstructionScript
  (Variables|DoorStates|SetInitialState (select (Utilities|Enum|Equal(Enum) (Variables|DoorStates|GetInitialState) "NewEnumerator3") "NewEnumerator1" (Variables|DoorStates|GetInitialState)))
  (bind _output_get (Variables|DoorStates|SetCurrentState (Variables|DoorStates|GetInitialState)))
  (CallFunction|Animate (Utilities|Select :Index _output_get :NewEnumerator0 1.0 :NewEnumerator1 0.0 :NewEnumerator2 0.0 :NewEnumerator3 0.0))
  (Variables|/Game/Keys/BPAC_Lock.BPAC_Lock_C|SetIsLoked (Variables|Default|GetBPAC_Lock) (Utilities|IsCurrentState "NewEnumerator2")))

(fn Close
  (Utilities|SwitchCurrentStateOld
    (:Opened
      (Variables|DoorStates|SetCurrentState "NewEnumerator3"))
    (:Closed
      (return false))
    (:Locked
      (return false))
    (:Transition
      (Utilities|SwitchTargetStateOld
        (:Opened
          _)
        (:Closed
          (return false))
        (:Locked
          (return false))
        (:Transition
          (return false)))))
  (Variables|DoorStates|SetTargetState "NewEnumerator1")
  (Utilities|String|Reverse (Variables|Default|GetDoorTimeline))
  (return true))

(fn Open
  (Utilities|SwitchCurrentStateOld
    (:Opened
      _)
    (:Closed
      (Variables|DoorStates|SetCurrentState "NewEnumerator3")
      (Variables|DoorStates|SetTargetState "NewEnumerator0" :!label _label)
      (Audio|Components|Audio|Play (Variables|Default|GetDoorTimeline))
      (return true))
    (:Locked
      _)
    (:Transition
      (Utilities|SwitchTargetStateOld
        (:Opened
          _)
        (:Closed
          (goto _label))
        (:Locked
          _)
        (:Transition
          _))
      (return false)))
  (return false))

(fn Animate
  (params (AnimationProgress :type Float%20%28double-precision%29))
  (Transformation|SetRelativeRotation (Variables|Default|GetDoorRotator) (Math|Rotator|MakeRotator 0.0 0.0 (* (Variables|Default|GetMaxDoorOpenAngle) AnimationProgress)) false false))

(fn SetIsLocked
  (params (OtherActor :type Actor%20Object%20Reference) (IsLocked :type Boolean))
  (if IsLocked
    (if (Utilities|IsCurrentState "NewEnumerator1")
      (bind _success (Default|Lock (Variables|Default|GetBPAC_Lock) OtherActor))
      (if _success
        (Variables|DoorStates|SetCurrentState "NewEnumerator2")
        (return true)
        (else
          (return false)))
      (else
        _))
    (elif (Utilities|IsCurrentState "NewEnumerator2")
      (bind _success_2 (Default|Unlock (Variables|Default|GetBPAC_Lock) OtherActor))
      (if _success_2
        (Variables|DoorStates|SetCurrentState "NewEnumerator1")
        (return true)
        (else
          (return false)))
      (else
        _)))
  (return false))

(fn GetCurrentState
  (return (Variables|DoorStates|GetCurrentState)))

(fn GetTargetState
  (return (Variables|DoorStates|GetTargetState)))

(fn Interact
  (params (Interactor :type Actor%20Object%20Reference))
  (return false))