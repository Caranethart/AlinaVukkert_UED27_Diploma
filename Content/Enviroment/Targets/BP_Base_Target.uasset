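; Base damageable target actor that tracks health and is destroyed when it runs out.
; AnyDamage passes damage to TakeDamage, which truncates it to an integer, subtracts it from the BPACHealth component and destroys the actor at zero or below.
; Every tick, a debug string at the actor's location shows current and maximum HP.
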(event EventTick
  (params (DeltaSeconds :type Float%20%28single-precision%29))
  (bind _bpac_health (Variables|Default|GetBPAC_Health))
  (Rendering|Debug|DrawDebugString (Transformation|GetActorLocation self) (Utilities|String|ToString(Text) (Utilities|Text|FormatText "{Name} HP : {Current} / {Max}" 0 (Default|GetCurrentValue _bpac_health) (Variables|/Game/Components/BPAC_EntityResourceBase.BPAC_EntityResourceBase_C|GetMaxValue _bpac_health))) 0 "(R=1.000000,G=0.033376,B=0.000000,A=1.000000)"))

(event Game|Damage|EventAnyDamage
  (params (Damage :type Float%20%28single-precision%29) (DamageType :type Damage%20Type%20Object%20Reference) (InstigatedBy :type Controller%20Object%20Reference) (DamageCauser :type Actor%20Object%20Reference))
  (CallFunction|TakeDamage Damage))

(fn ConstructionScript)

(fn TakeDamage
  (params (Amount :type Float%20%28double-precision%29))
  (Default|DecreaseValue (Variables|Default|GetBPAC_Health) (Math|Float|Truncate Amount))
  (if (<= (Default|GetCurrentValue (Variables|Default|GetBPAC_Health)) 0)
    (Actor|DestroyActor)
    (return)
    (else
      (return))))